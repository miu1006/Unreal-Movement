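; BP_Mirror is a mirror actor that captures the player's skeletal pose as 2D points and sends it to a local fencing pose server.
; CapturePose projects bone transforms onto the planar reflection, zooms them to a canvas and POSTs them as JSON through VaRest.
; Captures are numbered in batches of five steps, and the response callback calls OnPoseSent.
; Tick only advances a counter, as its timed capture check is disconnected.
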(event Custom|SentPoses
  (params (Request :type Va%20Rest%20Request%20JSON%20Object%20Reference))
  (Default|CallOnPoseSent))

(event Custom|CapturePose
  (bind _canvassize (Variables|Default|GetcanvasSize))
  (bind _joints (CallFunction|GetSkeletalPosSet (Variables|Default|GetskeletalMesh) (Variables|Default|Getplayer)))
  (for (_array_element _array_index) _joints
    (bind (_x _y) (CallFunction|GetPlaneProjection (Variables|Default|Getx) (Variables|Default|Gety) (Variables|Default|GetPlanarReflection) _array_element (Variables|Default|GetpixelDensity)))
    (CallFunction|AddtoOpenPoseArray _x _y 1.0 (Variables|Default|GetposesOnMirror) _array_index)
    (Development|PrintString (Utilities|String|ToString(Vector2d) (Math|Vector2D|MakeVector2D _x _y))))
  (bind _poseszoomed (CallFunction|GetZoomedArea (Variables|Default|GetposesOnMirror) (Variables|Default|GetcanvasSize)))
  (bind _output_get (Variables|Default|SetposesZoomed _poseszoomed))
  (Class|VaRestSubsystem|CallURL (|VaRestSubsystem) "localhost:5000/expo_fencing_pose" "POST" "json" (|MakeJson _output_get (Utilities|Array|MakeArray _canvassize _canvassize) (Math|Conversions|ToFloat(Integer) (Variables|Default|Getbatch)) (Math|Conversions|ToFloat(Integer) (Variables|Default|Getstep))) (delegate Custom|SentPoses))
  (bind _output_get_2 (Variables|Default|Setstep (+ (Variables|Default|Getstep) 1)))
  (if (> _output_get_2 4)
    (Variables|Default|Setstep 0)
    (Variables|Default|Setbatch (+ (Variables|Default|Getbatch) 1))))

(event EventBeginPlay
  (Variables|Default|SetskeletalMesh (Variables|/Game/OculusRetargeting/UnrealManequin/BP_FencingLiveLinkRetarget.BP_FencingLiveLinkRetarget_C|GetTargetRetargetMesh (Variables|Default|Getplayer))))

(event EventTick
  (params (DeltaSeconds :type Float%20%28single-precision%29))
  (Utilities|FlowControl|Sequence
    (:then_1
      (Variables|Default|Setcounter (Math|Float|%(Float) (+ DeltaSeconds (Variables|Default|Getcounter)) 1.0)))))

(fn ConstructionScript)

(fn ResetCaptureEvent
  (Variables|Default|Setbatch 0)
  (Variables|Default|Setstep 0))
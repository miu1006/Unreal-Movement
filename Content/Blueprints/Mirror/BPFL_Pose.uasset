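; Blueprint function library that turns a character's skeleton into OpenPose-style 2D keypoints on a mirror plane.
; GetSkeletalPosSet gathers socket locations, adding head-attached components for nose and ears, and draws debug spheres.
; GetPlaneProjection maps a world point to pixels using reference components and plane projections.
; AddToOpenPoseArray packs X, Y, confidence triplets, which GetZoomedArea rescales into a padded square crop at canvas size.
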(fn GetPlaneProjection
  (params (xRef :type Scene%20Component%20Object%20Reference) (yRef :type Scene%20Component%20Object%20Reference) (frontRef :type Scene%20Component%20Object%20Reference) (worldTransform :type Vector) (pixelDensity :type Float%20%28double-precision%29))
  (bind _returnvalue (Math|Vector|GetForwardVector frontRef))
  (bind _returnvalue_2 (Math|Vector|RotateVectorAroundAxis _returnvalue 9e+01 "0.000000,1.000000,0.000000"))
  (bind _returnvalue_3 (Math|Vector|ProjectVectorontoPlane worldTransform _returnvalue_2))
  (return (* (Math|Float|Absolute(Float) (.Y (Math|Vector|BreakVector (- (Math|Vector|ProjectVectorontoPlane _returnvalue_3 (Math|Vector|GetForwardVector xRef)) (Math|Vector|ProjectVectorontoPlane (Transformation|GetWorldLocation xRef) _returnvalue_2))))) pixelDensity) (* (Math|Float|Absolute(Float) (.Z (Math|Vector|BreakVector (- (Math|Vector|ProjectVectorontoPlane _returnvalue_3 (Math|Vector|GetForwardVector yRef)) (Math|Vector|ProjectVectorontoPlane (Transformation|GetWorldLocation yRef) _returnvalue_2))))) pixelDensity)))

(fn GetZoomedArea
  (params (posesOnMirror :type Array%20of%20Floats%20%28double-precision%29) (canvasSize :type Float%20%28double-precision%29))
  (Utilities|FlowControl|Sequence
    (:then_0
      (for (_array_element _array_index) posesOnMirror
        (Development|PrintString 0 (Utilities|String|ToString(Float) _array_element))
        (if (== (Math|Integer|%(Integer) _array_index 3) 0)
          (if (< _array_element (LocalVariables|GetminX))
            (LocalVariables|SetminX _array_element)
            (elif (> _array_element (LocalVariables|GetmaxX))
              (LocalVariables|SetmaxX _array_element)))
          (elif (== (Math|Integer|%(Integer) _array_index 3) 1)
            (if (< _array_element (LocalVariables|GetminY))
              (LocalVariables|SetminY _array_element)
              (elif (> _array_element (LocalVariables|GetmaxY))
                (LocalVariables|SetmaxY _array_element)))))))
    (:then_1
      (LocalVariables|SethalfWidth (* (Math|Float|Max(Float) (- (LocalVariables|GetmaxX) (LocalVariables|GetminX)) (- (LocalVariables|GetmaxY) (LocalVariables|GetminY))) 0.625))
      (LocalVariables|Set_centerX (/ (+ (LocalVariables|GetmaxX) (LocalVariables|GetminX)) 2.0))
      (LocalVariables|Set_centerY (/ (+ (LocalVariables|GetmaxY) (LocalVariables|GetminY)) 2.0))
      (LocalVariables|SetminX (- (LocalVariables|Get_centerX) (LocalVariables|GethalfWidth)))
      (LocalVariables|SetminY (- (LocalVariables|Get_centerY) (LocalVariables|GethalfWidth)))
      (LocalVariables|SetmaxX (+ (LocalVariables|Get_centerX) (LocalVariables|GethalfWidth)))
      (LocalVariables|SetmaxY (+ (LocalVariables|Get_centerY) (LocalVariables|GethalfWidth))))
    (:then_2
      (for _index (range 0 (- (Utilities|Array|Length posesOnMirror) 1))
        (if (== (Math|Integer|%(Integer) _index 3) 0)
          (Utilities|Array|SetArrayElem (LocalVariables|Get_posesZoomed) _index (* (/ (- (Utilities|Array|Get(acopy) posesOnMirror _index) (LocalVariables|GetminX)) (* (LocalVariables|GethalfWidth) 2.0)) canvasSize) true)
          (elif (== (Math|Integer|%(Integer) _index 3) 1)
            (Utilities|Array|SetArrayElem (LocalVariables|Get_posesZoomed) _index (* (/ (- (Utilities|Array|Get(acopy) posesOnMirror _index) (LocalVariables|GetminY)) (* (LocalVariables|GethalfWidth) 2.0)) canvasSize) true)
            (else
              (Utilities|Array|SetArrayElem (LocalVariables|Get_posesZoomed) _index 1.0 true))))))
    (:then_3
      (return (LocalVariables|Get_posesZoomed) (LocalVariables|Get_centerX) (LocalVariables|Get_centerY)))))

(fn AddtoOpenPoseArray
  (params (x :type Float%20%28double-precision%29) (y :type Float%20%28double-precision%29) (confidence :type Float%20%28double-precision%29) (outArray :type Array%20of%20Floats%20%28double-precision%29) (index :type Integer))
  (bind _returnvalue (* index 3))
  (bind _returnvalue_2 (+ _returnvalue 1))
  (Utilities|Array|SetArrayElem outArray _returnvalue x true)
  (Utilities|Array|SetArrayElem outArray _returnvalue_2 y true)
  (Utilities|Array|SetArrayElem outArray (+ _returnvalue_2 1) confidence true))

(fn GetSkeletalPosSet
  (params (skeletalMesh :type Skeletal%20Mesh%20Component%20Object%20Reference%20%28by%20ref%29) (target :type Actor%20Object%20Reference%20%28by%20ref%29))
  (Utilities|FlowControl|Sequence
    (:then_0
      (if (not (Utilities|IsValid (LocalVariables|Getnose)))
        (bind _returnvalue (Game|AddComponentbyClass target "/Script/Engine.SceneComponent" false (Math|Transform|MakeTransform "7.000000,-10.000000,0.000000")))
        (Transformation|AttachComponentToComponent _returnvalue skeletalMesh "Head" "KeepRelative" "KeepRelative" "KeepRelative" true)
        (LocalVariables|Setnose _returnvalue)))
    (:then_1
      (if (not (Utilities|IsValid (LocalVariables|GetleftEar)))
        (bind _returnvalue_2 (Game|AddComponentbyClass target "/Script/Engine.SceneComponent" false (Math|Transform|MakeTransform "10.000000,0.000000,7.000000")))
        (Transformation|AttachComponentToComponent _returnvalue_2 skeletalMesh "Head" "KeepRelative" "KeepRelative" "KeepRelative" true)
        (LocalVariables|SetleftEar _returnvalue_2)))
    (:then_2
      (if (not (Utilities|IsValid (LocalVariables|GetrightEar)))
        (bind _returnvalue_3 (Game|AddComponentbyClass target "/Script/Engine.SceneComponent" false (Math|Transform|MakeTransform "10.000000,0.000000,-7.000000")))
        (Transformation|AttachComponentToComponent _returnvalue_3 skeletalMesh "Head" "KeepRelative" "KeepRelative" "KeepRelative" true)
        (LocalVariables|SetrightEar _returnvalue_3)))
    (:then_3
      (for _array_element (LocalVariables|GetjonitNames)
        (Utilities|Array|Add (LocalVariables|GettempJoints) (Transformation|GetSocketLocation skeletalMesh (Utilities|String|StringToName _array_element)))
        (Rendering|Debug|DrawDebugSphere 0 (Transformation|GetSocketLocation skeletalMesh (Utilities|String|StringToName _array_element)) 1.0 12 "(R=1.000000,G=0.000000,B=0.000000,A=1.000000)" 1.0 1.0))
      (Utilities|Array|SetArrayElem (LocalVariables|GettempJoints) (Utilities|Array|FindItem (LocalVariables|GetjonitNames) "Nose") (Transformation|GetWorldLocation (LocalVariables|Getnose)))
      (Utilities|Array|SetArrayElem (LocalVariables|GettempJoints) (Utilities|Array|FindItem (LocalVariables|GetjonitNames) "LeftEar") (Transformation|GetWorldLocation (LocalVariables|GetleftEar)))
      (Utilities|Array|SetArrayElem (LocalVariables|GettempJoints) (Utilities|Array|FindItem (LocalVariables|GetjonitNames) "RightEar") (Transformation|GetWorldLocation (LocalVariables|GetrightEar)))
      (Rendering|Debug|DrawDebugSphere 0 (Transformation|GetWorldLocation (LocalVariables|Getnose)) 1.0 12 "(R=0.000000,G=0.000000,B=1.000000,A=1.000000)" 1.0 0.1)
      (Rendering|Debug|DrawDebugSphere 0 (Transformation|GetWorldLocation (LocalVariables|GetleftEar)) 1.0 12 "(R=0.000000,G=0.000000,B=1.000000,A=1.000000)" 1.0 0.1)
      (Rendering|Debug|DrawDebugSphere 0 (Transformation|GetWorldLocation (LocalVariables|GetrightEar)) 1.0 12 "(R=0.000000,G=0.000000,B=1.000000,A=1.000000)" 1.0 0.1)
      (return (LocalVariables|GettempJoints)))))